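; Player character Blueprint for a runner tag game that adds a timed speed boost with a cooldown.
; IA_Boost multiplies the walk speed cached at BeginPlay, starts duration and cooldown timers together, and sets cooldown state variables.
; EndBoost restores speed and clears CanBoost until ResetBoost re-enables it, with printed status messages.
; CanBoost stays true during a boost, so pressing again restarts both timers.
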(event Custom|EndBoost
  ;[0.8854 0 1] End Of The Boost (Boost is charing and can not be used)
  (Variables|Default|SetbCanBoost false)
  (Variables|/Script/Engine.CharacterMovementComponent|SetMaxWalkSpeed (Variables|Character|GetCharacterMovement) (Variables|Default|GetBaseWalkSpeed)))

(event Custom|ResetBoost
  ;[0 1 0.03201] Boost Reset & String For Player (Boost has reset and ready to use)
  (Variables|Default|SetbCanBoost true)
  (Development|PrintString "Boost Is Now Ready"))

(event Input|EnhancedActionEvents|EnhancedInputActionIA_Boost
  (params (ActionValue :type Boolean) (ElapsedSeconds :type Float%20%28double-precision%29) (TriggeredSeconds :type Float%20%28double-precision%29) (InputAction :type Input%20Action%20Object%20Reference :default "/Game/ThirdPerson/Input/Actions/IA_Boost.IA_Boost"))
  ;[1 0.1823 0.1823] Boost Input
  (:Started
    (if (Variables|Default|GetbCanBoost)
      (Variables|Default|SetbCanBoost true)
      (Variables|/Script/Engine.CharacterMovementComponent|SetMaxWalkSpeed (Variables|Character|GetCharacterMovement) (* (Variables|Default|GetBoostMultiplier) (Variables|Default|GetBaseWalkSpeed)))
      (Utilities|Time|SetTimerbyFunctionName 0 "EndBoost" (Variables|Default|GetBoostDuration))
      (Utilities|Time|SetTimerbyFunctionName 0 "ResetBoost" (Variables|Default|GetBoostCooldown))
      (Variables|Default|SetBoostCooldownRemaining (Variables|Default|GetBoostCooldown))
      (Variables|Default|SetbIsCooldownActive true)
      (else
        (Development|PrintString "Boost Is Still Charging")))))

(event EventBeginPlay
  ;[0 0.04666 1] Base Walk Speed When Game Starts
  (Variables|Default|SetBaseWalkSpeed (Variables|/Script/Engine.CharacterMovementComponent|GetMaxWalkSpeed (Variables|Character|GetCharacterMovement))))

(fn ConstructionScript)